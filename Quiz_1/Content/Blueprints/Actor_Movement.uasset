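; Actor that moves itself on the horizontal plane from player input, enabled for player controller 0 on BeginPlay.
; Each Tick builds an X/Y vector from the Horizontal and Vertical values, multiplies it by Speed and adds it to the actor's location.
; The step is not scaled by delta time, so speed depends on frame rate, and it is set without sweep, so collisions do not block it.
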(event EventTick
  (params (DeltaSeconds :type Float%20%28single-precision%29))
  (Transformation|SetActorLocation (+ (* (Math|Vector|MakeVector (Input|AxisValues|GetHorizontal) (Input|AxisValues|GetVertical) 0.0) (Variables|Default|GetSpeed)) (Transformation|GetActorLocation)) false false))

(event EventBeginPlay
  (Input|EnableInput (Game|GetPlayerController 0)))

(fn ConstructionScript)